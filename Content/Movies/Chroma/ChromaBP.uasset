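; ChromaBP is an actor that displays a chroma material, judging by its names, either on a camera-facing material billboard or on a static mesh.
; The construction script toggles visibility between the two components from the Bilboard flag.
; In billboard mode it prints the scaled base size and, when TestSize is set, writes that size and the ChromaMat_Inst material into the first billboard element.
; The event graph holds no active logic.
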(fn `UserConstructionScript`
  (bind _materialbillboard (`self.MaterialBillboard`))
  (bind _staticmesh (`self.StaticMesh`))
  (bind _scale (`self.Scale`))
  (bind _returnvalue (* (`self.Base Size Y`) _scale))
  (bind _returnvalue_2 (* (`self.Base Size X`) _scale))
  (if (`self.Bilboard?`)
    (`SceneComponent.SetVisibility` _materialbillboard true false)
    (`SceneComponent.SetVisibility` _staticmesh false false)
    (`KismetSystemLibrary.PrintString` (`KismetStringLibrary.Concat_StrStr` (`KismetStringLibrary.Conv_DoubleToString` _returnvalue_2) " X " (`KismetStringLibrary.Conv_DoubleToString` _returnvalue)))
    (if (`self.TestSize`)
      (setmembers `MaterialSpriteElement` :`StructRef` (`|GetArrayItem` (`MaterialBillboardComponent.Elements` (`self.MaterialBillboard`))) :`Material` "/Game/Movies/Chroma/ChromaMat_Inst.ChromaMat_Inst" :`BaseSizeX` _returnvalue_2 :`BaseSizeY` _returnvalue))
    (else
      (`SceneComponent.SetVisibility` _staticmesh true false)
      (`SceneComponent.SetVisibility` _materialbillboard false false))))