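; Builder Blueprint that lays out static mesh components along a circular arc when Generate is set.
; Mode derives count and angular step from amount, angle or arch span, with cumulative offsets, optional facing and seeded random transform variation.
; Meshes cycle or are picked randomly, then SpecificMeshes overrides individual indices' mesh and transform.
; PlacePermanentCopies spawns each generated piece as a standalone StaticMeshActor.
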(fn `PlacePermanentCopies`
  (for _array_element (`self.MeshComps`)
    (bind _returnvalue (`|SpawnActorFromClass` "/Script/Engine.StaticMeshActor" (`SceneComponent.K2_GetComponentToWorld` _array_element) "AlwaysSpawn" "OverrideRootScale" null null))
    (`StaticMeshComponent.SetStaticMesh` (`StaticMeshActor.StaticMeshComponent` _returnvalue) (`StaticMeshComponent.StaticMesh` _array_element))))

(fn `UserConstructionScript`
  (bind _angle (`self.Angle`))
  (bind _locationbase (`self.LocationBase`))
  (bind _mesh (`self.Mesh`))
  (bind _archangle (`self.ArchAngle`))
  (bind _angle_2 (`self.Angle`))
  (bind _seed (`self.Seed`))
  (bind _returnvalue (`KismetArrayLibrary.Array_Length` _mesh))
  (if (`self.Generate`)
    (`KismetArrayLibrary.Array_Clear` (`self.MeshComps`))
    (`|ExecutionSequence`
      (:`then_0`
        (for _index (range (+ (select `/Game/Builder/Blueprints/EArchPlacement` (`self.Mode`) :`NewEnumerator0` (- (`self.Amount`) 1) :`NewEnumerator1` (- (`self.Amount`) 1) :`NewEnumerator2` (`KismetMathLibrary.FFloor` (/ _archangle (`KismetMathLibrary.SelectFloat` _archangle _angle_2 (== _angle_2 0.0))))) 1))
          (bind _returnvalue_2 (+ (`self.BaseAngle`) (* _index (select `/Game/Builder/Blueprints/EArchPlacement` (`self.Mode`) :`NewEnumerator0` _angle :`NewEnumerator1` (/ (`self.ArchAngle`) (`KismetMathLibrary.Conv_IntToDouble` (`KismetMathLibrary.Max` (`self.Amount`) 1))) :`NewEnumerator2` _angle))))
          (bind _returnvalue_3 (`AddComponent|NODE_AddStaticMeshComponent-0` :`RelativeTransform` (`/Game/Builder/Blueprints/BP_FuncLib.CombineTransform` (`KismetMathLibrary.MakeTransform` (+ (`KismetMathLibrary.SelectVector` _locationbase (+ (`KismetMathLibrary.MakeVector` 0.0 (* (`self.Radius`) -1.0)) _locationbase) (`self.Center`)) (* (`KismetMathLibrary.MakeVector` (`KismetMathLibrary.DegCos` _returnvalue_2) (`KismetMathLibrary.DegSin` _returnvalue_2)) (`self.Radius`)) (* (`self.LocationOffset`) _index)) (`KismetMathLibrary.ComposeRotators` (`KismetMathLibrary.SelectRotator` (`KismetMathLibrary.MakeRotator` 0.0 0.0 _returnvalue_2) (* (`self.RotationOffset`) _index) (`self.FaceCenter`)) (`self.RotationBase`)) (+ (* (`self.ScaleOffset`) _index) (`self.ScaleBase`))) (`KismetMathLibrary.MakeTransform` (`/Game/Builder/Blueprints/BP_FuncLib.RandomVectorSeeded` (`self.MinRandomLocation`) (`self.MaxRandomLocation`) _seed) (`/Game/Builder/Blueprints/BP_FuncLib.RandomRotSeeded` (`self.MinRandomRotation`) (`self.MaxRandomRotation`) _seed) (`/Game/Builder/Blueprints/BP_FuncLib.RandomVectorSeeded` (`self.MinRandomScale`) (`self.MaxRandomScale`) _seed)))))
          (`StaticMeshComponent.SetStaticMesh` _returnvalue_3 (select `/Game/Builder/Blueprints/ESelect` (`self.MeshSelection`) :`NewEnumerator0` (`|GetArrayItem` _mesh (mod _index _returnvalue)) :`NewEnumerator1` (`|GetArrayItem` _mesh (`KismetMathLibrary.RandomIntegerFromStream` _returnvalue (`self.Seed`)))))
          (`KismetArrayLibrary.Array_Add` (`self.MeshComps`) _returnvalue_3)))
      (:`then_1`
        (for _array_element (`self.SpecificMeshes`)
          (bind (_index_2 _mesh_2 _offset _rot _scale) (break `/Game/Builder/Blueprints/S_IndexMesh` _array_element))
          (if (and (> (`KismetArrayLibrary.Array_Length` (`self.MeshComps`)) _index_2) (> _index_2 -1))
            (bind _output (`|GetArrayItem` (`self.MeshComps`) _index_2))
            (`StaticMeshComponent.SetStaticMesh` _output _mesh_2)
            (`SceneComponent.K2_SetRelativeTransform` _output (`KismetMathLibrary.MakeTransform` (+ (`SceneComponent.RelativeLocation` _output) _offset) _rot _scale) false false)))))))