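; Builder actor that, judging by its name, is meant to stack meshes along a linear spline, though it currently places none.
; When Generate is set, the construction script sizes the scale arrays to Meshes and Connectors, defaulting zero scales to one.
; It makes every spline point linear and applies the Loop setting.
; The final per-segment loop is empty, and MeshSelection and Seed are unused.
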(fn `UserConstructionScript`
  (bind _loop (`self.Loop`))
  (bind _returnvalue (`SplineComponent.GetNumberOfSplinePoints` (`self.Spline`)))
  (if (`self.Generate`)
    (`|ExecutionSequence`
      (:`then_1`
        (`|ExecutionSequence`
          (:`then_0`
            (`KismetArrayLibrary.Array_Resize` (`self.MeshScales`) (`KismetArrayLibrary.Array_Length` (`self.Meshes`)))
            (`KismetArrayLibrary.Array_Resize` (`self.ConnectorScales`) (`KismetArrayLibrary.Array_Length` (`self.Connectors`)))
            (`|ExecutionSequence`
              (:`then_0`
                (for (_array_element _array_index) (`self.MeshScales`)
                  (if (== _array_element (0.0 0.0 0.0))
                    (`KismetArrayLibrary.Array_Set` (`self.MeshScales`) _array_index (1.0 1.0 1.0)))))
              (:`then_1`
                (for (_array_element_2 _array_index_2) (`self.ConnectorScales`)
                  (if (== _array_element_2 (0.0 0.0 0.0))
                    (`KismetArrayLibrary.Array_Set` (`self.ConnectorScales`) _array_index_2 (1.0 1.0 1.0)))))))
          (:`then_1`
            (for _index (range (`SplineComponent.GetNumberOfSplinePoints` (`self.Spline`)))
              (`SplineComponent.SetSplinePointType` (`self.Spline`) _index "Linear" false)))
          (:`then_2`
            (`SplineComponent.SetClosedLoop` (`self.Spline`) _loop true)
            (`|ExecutionSequence`
              (:`then_0`
                (for _ (range 1 (+ (`KismetMathLibrary.SelectInt` _returnvalue (- _returnvalue 1) _loop) 1))
                  _)))))))))