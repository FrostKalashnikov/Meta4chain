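; Blueprint that plays a timed, sequential showcase of skeletal mesh and animation pairs, despite "Random" in its name.
; On BeginPlay it starts the sequence and prints the summed length of all animations.
; ChangeMeshNAnim uses a DoN counter, capped at 20, to index parallel mesh and animation arrays.
; It swaps the mesh, plays the clip once, prints its details, then re-triggers itself after the clip's length.
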(event `self.ReceiveBeginPlay`
  (`self.ChangeMesh N Anim`)
  (for _array_element (`self.AllAnimation`)
    (set `self.TotalTime` (+ (`self.TotalTime`) (`AnimationAsset.GetPlayLength` _array_element))))
  (`KismetSystemLibrary.PrintString` (`KismetStringLibrary.Conv_DoubleToString` (`self.TotalTime`))))

(event `ChangeMesh N Anim`
  (bind _skeletalmesh (`self.SkeletalMesh`))
  (bind _counter (`/Engine/EditorBlueprintResources/StandardMacros.Do N` 20)
    (:`Exit`
      (bind _output (`|GetArrayItem` (`self.AllMeshes`) _counter))
      (`SkinnedMeshComponent.SetSkinnedAssetAndUpdate` _skeletalmesh _output true)
      (bind _output_2 (`|GetArrayItem` (`self.AllAnimation`) _counter))
      (`SkeletalMeshComponent.PlayAnimation` _skeletalmesh _output_2 false)
      (bind _returnvalue (`AnimationAsset.GetPlayLength` _output_2))
      (`KismetSystemLibrary.PrintString` (`KismetStringLibrary.Concat_StrStr` "Mesh: " (`KismetSystemLibrary.GetDisplayName` _output) " Anim: " (`KismetSystemLibrary.GetDisplayName` _output_2) " Length: " (`KismetStringLibrary.Conv_DoubleToString` _returnvalue)) true true (struct :`G` 0.66 :`B` 1.0 :`A` 1.0) _returnvalue)
      (`KismetSystemLibrary.Delay` _returnvalue)
      (`self.ChangeMesh N Anim`))))

(fn `UserConstructionScript`)