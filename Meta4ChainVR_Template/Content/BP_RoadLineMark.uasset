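; Spline-driven actor that lays a static mesh along a path, by its name for painting road line markings.
; The construction script truncates spline length over mesh length to get a segment count, then spreads the segments evenly across the whole spline.
; Each segment is a spline mesh component with tangents normalized and scaled to segment length, so the mesh follows the curve.
; It has no active runtime logic.
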(fn `UserConstructionScript`
  (bind _spline (`self.Spline`))
  (bind _segment_index (`self.Segment Index`))
  (bind _curve_tangent (`self.Curve Tangent`))
  (bind _curve_tangent_2 (`self.Curve Tangent`))
  (bind _number_of_segments (`self.Number of Segments`))
  (bind _returnvalue (`SplineComponent.GetSplineLength` (`self.Spline`)))
  (bind _returnvalue_2 (* _segment_index _curve_tangent))
  (bind _returnvalue_3 (* (+ _segment_index 1) _curve_tangent))
  (set `self.Number of Segments` (`KismetMathLibrary.FTrunc` (/ _returnvalue (`self.Mesh Lenght`))))
  (set `self.Curve Tangent` (/ _returnvalue (`KismetMathLibrary.Conv_IntToDouble` _number_of_segments)))
  (for _index (range _number_of_segments)
    (set `self.Segment Index` _index)
    (bind _returnvalue_4 (`AddComponent|NODE_AddSplineMeshComponent-0`))
    (`StaticMeshComponent.SetStaticMesh` _returnvalue_4 (`self.Static Mesh`))
    (`SplineMeshComponent.SetStartAndEnd` _returnvalue_4 (`SplineComponent.GetLocationAtDistanceAlongSpline` _spline _returnvalue_2 "Local") (* (`KismetMathLibrary.Normal` (`SplineComponent.GetTangentAtDistanceAlongSpline` _spline _returnvalue_2 "Local")) _curve_tangent_2) (`SplineComponent.GetLocationAtDistanceAlongSpline` _spline _returnvalue_3 "Local") (* (`KismetMathLibrary.Normal` (`SplineComponent.GetTangentAtDistanceAlongSpline` _spline _returnvalue_3 "Local")) _curve_tangent_2) true)))