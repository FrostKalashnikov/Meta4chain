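; AI pawn Blueprint that walks an endless looping route through the actors in its PathLocations array.
; On BeginPlay it picks a random skeletal mesh from AllMeshes, then starts moving after a short delay.
; AIMoveTo targets the current point, and both success and failure advance the index, wrapping to zero, before moving again.
; Only the starting point is checked for validity.
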(event `self.ReceiveBeginPlay`
  (`parent.ReceiveBeginPlay`)
  (`SkinnedMeshComponent.SetSkinnedAssetAndUpdate` (`self.Mesh`) (`KismetArrayLibrary.Array_Random` (`self.AllMeshes`)) true)
  (`KismetSystemLibrary.Delay` 0.2)
  (`self.GoToLocation`))

(event `GoToLocation`
  (bind _output (`|GetArrayItem` (`self.PathLocations`) (`self.LocID`)))
  (`/Engine/EditorBlueprintResources/StandardMacros.IsValid` _output
    (:`Is Valid`
      (`|AIMoveTo` self (`self.K2_GetActorLocation` _output) null 50.0 :!label _label
        (:`OnSuccess`
          _)
        (:`OnFail`
          _))
      (`|ExecutionSequence`
        (:`then_0`
          (if (`KismetArrayLibrary.Array_IsValidIndex` (`self.PathLocations`) (+ (`self.LocID`) 1))
            (`/Engine/EditorBlueprintResources/StandardMacros.IncrementInt` (`self.LocID`))
            (else
              (set `self.LocID` 0))))
        (:`then_1`
          (goto _label))))))

(fn `UserConstructionScript`
  (`parent.UserConstructionScript`))