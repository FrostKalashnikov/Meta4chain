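; VR trigger area that shows a text prompt and lets the player board a spline-driven VLT, use a teleport portal or toggle a drone sequence.
; Box overlap toggles input and the prompt, optionally turned toward the player on Tick through a gate.
; B or Interact runs whichever actions have valid references.
; VLT door changes drive availability; boarding switches view target, and exiting restores it and moves the pawn to the VRLOC component.
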(event `Passeio VLT`
  (params (`Open?` :type Boolean))
  (set `self.CanInteract` `Open?`)
  (`self.Sair VLT`)
  (if (`self.IsOverlappingActor` (`GameplayStatics.GetPlayerPawn` 0))
    (`SceneComponent.SetHiddenInGame` (`self.TextRender`) (not `Open?`) true)))

(event `self.ReceiveBeginPlay`
  (bind _vlt_splineref (`self.VLT_SplineRef`)
    (:`then`
      (add `/Game/Assets_Exterior/vlt/VLT_SplineSpeed.OnDoorsChange` _vlt_splineref (`|CreateDelegate` :!event `Passeio VLT`)))
    (:`else`)))

(event `self.ReceiveTick`
  (params (DeltaSeconds :type "Float (single-precision)"))
  (`/Engine/EditorBlueprintResources/StandardMacros.Gate` true :!label _label
    (:`Exit`
      (`SceneComponent.K2_SetWorldRotation` (`self.TextRender`) (`KismetMathLibrary.FindLookAtRotation` (`self.K2_GetActorLocation`) (`self.K2_GetActorLocation` (`GameplayStatics.GetPlayerPawn` 0))) false false))))

(event `OpenRotText`
  (goto _label :!via `Open`))

(event `CloseRotText`
  (goto _label :!via `Close`))

(event `Sair VLT`
  (bind _returnvalue (`GameplayStatics.GetPlayerPawn` 0))
  (if (and (`self.InVLT`) (`self.CanInteract`))
    (`PlayerController.SetViewTargetWithBlend` (`GameplayStatics.GetPlayerController` 0) _returnvalue 0.0 "VTBlend_Linear" 0.0 false)
    (`self.K2_SetActorLocation` _returnvalue (`SceneComponent.K2_GetComponentLocation` (`|GetArrayItem` (`self.GetComponentsByTag` (`/Game/Assets_Exterior/vlt/VLT_SplineSpeed.Character Ref` (`self.VLT_SplineRef`)) "/Script/Engine.SceneComponent" "VRLOC"))) false false)
    (set `self.InVLT` false)
    (set `self.CanInteract` false)))

(event `self.Box.OnComponentBeginOverlap`
  (params (OverlappedComponent :type "PrimitiveComponent Object Reference") (OtherActor :type "Actor Object Reference") (OtherComp :type "PrimitiveComponent Object Reference") (OtherBodyIndex :type Integer) (bFromSweep :type Boolean) (SweepResult :type "HitResult Structure (by ref)"))
  (`self.IsPlayer?` OtherActor
    (:`true`
      (`self.EnableInput` (`GameplayStatics.GetPlayerController` 0))
      (if (`self.CanInteract`)
        (`SceneComponent.SetHiddenInGame` (`self.TextRender`) false true)
        (if (`self.RotateText?`)
          (`self.OpenRotText`))))))

(event `Entrar VLT`
  (bind _vlt_splineref (`self.VLT_SplineRef`)
    (:`then`
      (bind _character_ref (`/Game/Assets_Exterior/vlt/VLT_SplineSpeed.Character Ref` _vlt_splineref)
        (:`then`
          (`PlayerController.SetViewTargetWithBlend` (`GameplayStatics.GetPlayerController` 0) _character_ref 0.0 "VTBlend_Linear" 0.0 false)
          (set `self.InVLT` true)
          (set `self.CanInteract` false))
        (:`else`)))
    (:`else`)))

(event `self.Box.OnComponentEndOverlap`
  (params (OverlappedComponent :type "PrimitiveComponent Object Reference") (OtherActor :type "Actor Object Reference") (OtherComp :type "PrimitiveComponent Object Reference") (OtherBodyIndex :type Integer))
  (`self.IsPlayer?` OtherActor
    (:`true`
      (`self.DisableInput` (`GameplayStatics.GetPlayerController` 0))
      (`SceneComponent.SetHiddenInGame` (`self.TextRender`) true true)
      (`self.CloseRotText`))))

(event `UsarPortal`
  (bind _teleportref (`self.TeleportRef`)
    (:`then`
      (bind (_returnvalue_location _returnvalue_rotation) (`KismetMathLibrary.BreakTransform` (`self.GetTransform` _teleportref)))
      (`self.K2_SetActorLocationAndRotation` (`GameplayStatics.GetPlayerPawn` 0) _returnvalue_location _returnvalue_rotation false false))
    (:`else`)))

(event `Key|B`
  (params (Key :type "Key Structure"))
  (:`Pressed`
    (`KismetSystemLibrary.PrintString` (`KismetTextLibrary.Conv_TextToString` (`KismetInputLibrary.Key_GetDisplayName` Key)))
    (if (`self.CanInteract`) :!label _label_2
      (`self.Entrar VLT`)
      (`self.UsarPortal`)
      (`self.UsarDrone`))))

(event `InputAction|Interact`
  (params (Key :type "Key Structure"))
  (:`Pressed`
    (goto _label_2)))

(event `UsarDrone`
  (bind _droneseqref (`self.DroneSeqRef`)
    (:`then`
      (if (`self.CanInteract`)
        (if (`self.InVLT`)
          (bind _sequenceplayer (`LevelSequenceActor.SequencePlayer` _droneseqref))
          (`MovieSceneSequencePlayer.Stop` _sequenceplayer)
          (set `self.InVLT` false)
          (else
            (`MovieSceneSequencePlayer.Play` _sequenceplayer)
            (`self.CloseRotText`)
            (`SceneComponent.SetHiddenInGame` (`self.TextRender`) true true)
            (set `self.InVLT` true)))))
    (:`else`)))

(event `PausePreEnd`
  (`MovieSceneSequencePlayer.Pause` (`LevelSequenceActor.SequencePlayer` (stale `UsarDrone` _droneseqref))))

(fn `UserConstructionScript`)